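; BP_Ship is a ship Blueprint that manages the radar object belonging to the ship.
; UpdateRadarObject takes a RadarInfo, then either updates the existing BP_Radar or constructs a new one from it.
; An empty name in the info's general details clears the radar, a check the code marks as a temporary stand-in for explicit removal.
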(fn `UpdateRadarObject`
  (params (RadarInfo :type "/Game/Assets/Data/F_RadarComponent Structure (by ref)"))
  (bind _radar (`self.Radar`))
  (if (== (`KismetStringLibrary.Len` (`KismetTextLibrary.Conv_TextToString` (`.Name_10_55EE3B8D42F38D8C4AB2F4BD744DA81B` (break `/Game/Assets/Data/F_ComponentGeneralDetails` (`.GeneralDetails_2_4ED183B74E1793CBD18D579D67B5B4F8` (break `/Game/Assets/Data/F_RadarComponent` RadarInfo)))))) 0)
    (set `self.Radar` null)
    (elif (`KismetSystemLibrary.IsValid` _radar)
      (set `/Game/BPs/BP_Radar.RadarInfo` RadarInfo _radar)
      (else
        (bind _returnvalue (`|GenericCreateObject` "/Game/BPs/BP_Radar.BP_Radar_C" RadarInfo))
        (set `self.Radar` _returnvalue)))))