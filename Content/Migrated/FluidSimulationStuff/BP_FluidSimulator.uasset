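; BP_FluidSimulator couples a Niagara fluid simulation to a solid object, feeding simulation results back as forces on that object.
; At BeginPlay it passes the solid's mass and static mesh to the Niagara system and registers itself as the export callback handler.
; The particle data callback repurposes the first particle's Position, Velocity and Size as force, torque and delta time, scaling the two vectors before calling SetForces.
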(event `self.ReceiveBeginPlay`
  (bind _niagaracomponent (`self.NiagaraComponent`))
  (bind _staticmeshcomponent (`StaticMeshActor.StaticMeshComponent` (`.SolidObject` (`self.SolidObject`))))
  (`FXSystemComponent.SetFloatParameter` _niagaracomponent "SolidMass" (`PrimitiveComponent.GetMass` _staticmeshcomponent))
  (`NiagaraFunctionLibrary.OverrideSystemUserVariableStaticMeshComponent` _niagaracomponent "SolidObject" _staticmeshcomponent)
  (`NiagaraComponent.SetVariableObject` _niagaracomponent "BPCallBackHandler" self))

(event `self.ReceiveParticleData`
  (params (Data :type "Array of BasicParticleData Structure (by ref)") (NiagaraSystem :type "NiagaraSystem Object Reference") (SimulationPositionOffset :type "Vector Structure (by ref)"))
  (bind (_position _size _velocity) (break `BasicParticleData` (`|GetArrayItem` Data)))
  (bind _returnvalue (`KismetMathLibrary.Conv_DoubleToVector` (* 9.765625 1000.0)))
  (`self.Set Forces` (`.SolidObject` (`self.SolidObject`)) (* _position _returnvalue) (* _returnvalue _velocity) _size))

(fn `UserConstructionScript`)